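; Fireball projectile effect actor from FXVarietyPack, with its movement, lifetime and hit logic present but disconnected from the events.
; BeginPlay, Tick and ActorBeginOverlap are empty, so none of that logic runs.
; The unwired chains spawn a tinted shockwave, move along local X with timeline-corrected speed, and count down Duration before deactivating and destroying.
; An unwired overlap chain spawns HitFx and destroys the actor, ignoring "ky_shot"-tagged actors.
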(event EventBeginPlay
  ;[1 1 1] spawn shot shockwave
)

(event Collision|EventActorBeginOverlap
  (params (OtherActor :type Actor%20Object%20Reference))
  ;[1 1 1] spawn collison fx
)

(event EventTick
  (params (DeltaSeconds :type Float%20%28single-precision%29))
  ;[1 1 1] duration increment for control
)

(fn ConstructionScript)