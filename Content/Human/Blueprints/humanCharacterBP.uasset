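; Player human character Blueprint for a free-for-all spellshooter, handling look input and end-of-match screens.
; BeginPlay spawns a placeholder AK weapon so later weapon swaps can delete it, then binds the locally controlled player to the game state's winner-found event.
; Tick derives ControlPitch from control rotation on authority.
; Victory, death and winner-located handlers show widgets and the cursor; helpers expose weapon socket transforms and teleport the character onto existing character transforms.
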(event Custom|onWinPlayerFound_Event_0
  (bind _returnvalue (UserInterface|CreateWidget "/Game/Multiplayer/UI/playerWinnerLocScreenWidget.playerWinnerLocScreenWidget_C" (stale EventBeginPlay _asspellshooter_player_controller_bp)))
  (Variables|/Script/Engine.PlayerController|SetbShowMouseCursor (stale EventBeginPlay _asspellshooter_player_controller_bp) true)
  (UserInterface|Viewport|AddtoViewport _returnvalue 0)
  (Variables|Default|SetwinnerIsLocated true))

(event Custom|CustomEvent
  ;[1 1 1] ignore, backup of old logic, do not use
)

(event EventBeginPlay
  ;[1 0 0] THIS IS DUMB: Give player a "playerWeapon" actor (see c++ variable), otherwise engine complains when attempting to delete playerWeapon before equipping new weapon inside the "spellshooterPlayerController" component
  (bind _returnvalue (Game|SpawnActorfromClass "/Game/Weapons/Blueprints/akBP.akBP_C" (Math|Transform|MakeTransform "0.000000,-100.000000, 0" "0, 0, 0" "0.010000,0.010000,0.010000") "DontSpawnIfColliding" 0 0))
  (Variables|Default|SetplayerWeapon _returnvalue)
  (bind _asspellshooter_player_controller_bp (Utilities|Casting|CastTospellshooterPlayerControllerBP (Pawn|GetController)))
  (if (Pawn|IsLocallyControlled (Pawn|GetControlledPawn _asspellshooter_player_controller_bp))
    (bind _asffa_game_state (Utilities|Casting|CastToffaGameState (Game|GetGameState)))
    (EventDispatchers|BindEventtoOnWinPlayerFound _asffa_game_state (delegate Custom|onWinPlayerFound_Event_0))))

(event Collision|EventActorBeginOverlap
  (params (OtherActor :type Actor%20Object%20Reference)))

(event EventTick
  (params (DeltaSeconds :type Float%20%28single-precision%29))
  (bind _returnvalue (Pawn|GetControlRotation :!class /Script/Engine.Pawn))
  (bind _pitch (Math|Rotator|BreakRotator _returnvalue))
  (Utilities|FlowControl|Sequence
    (:then_0
      (Networking|SwitchHasAuthority
        (:Authority
          (Variables|Default|SetcontrolPitch (Math|Rotator|MakeRotator (/ (Math|Float|SelectFloat (- 3.6e+02 _pitch) (* _pitch -1.0) (> _pitch 1.8e+02)) 3.0) 0.0 0.0)))))))

(event EventDisplayDeathScreen
  (Variables|Default|SetisDead true)
  (bind _foundwidgets (Widget|GetAllWidgetsOfClass "/Game/Multiplayer/playerHUD/playerHPbarWidget.playerHPbarWidget_C" false))
  (Widget|RemovefromParent _foundwidgets)
  (bind _returnvalue (UserInterface|CreateWidget "/Game/Multiplayer/UI/playerDeathScreenWidget.playerDeathScreenWidget_C"))
  (bind _output_get (Variables|Default|SetonDeathRef _returnvalue))
  (bind _asspellshooter_player_controller_bp (Utilities|Casting|CastTospellshooterPlayerControllerBP (Pawn|GetController)))
  (Variables|/Script/Engine.PlayerController|SetbShowMouseCursor _asspellshooter_player_controller_bp true)
  (UserInterface|Viewport|AddtoViewport _output_get 0))

(event EventDisplayVictoryScreen
  (bind _foundwidgets (Widget|GetAllWidgetsOfClass "/Game/Multiplayer/playerHUD/playerHPbarWidget.playerHPbarWidget_C" false))
  (Widget|RemovefromParent _foundwidgets)
  (bind _returnvalue (UserInterface|CreateWidget "/Game/Multiplayer/UI/playerWinScreenWidget.playerWinScreenWidget_C"))
  (bind _output_get (Variables|Default|SetonWinRef _returnvalue))
  (bind _asspellshooter_player_controller_bp (Utilities|Casting|CastTospellshooterPlayerControllerBP (Pawn|GetController)))
  (Variables|/Script/Engine.PlayerController|SetbShowMouseCursor _asspellshooter_player_controller_bp true)
  (UserInterface|Viewport|AddtoViewport _output_get 0))

(event Input|AxisEvents|InputAxisTurn
  (params (AxisValue :type Float%20%28single-precision%29))
  (Variables|Default|SetbUseControllerRotationYaw true)
  (Pawn|Input|AddControllerYawInput AxisValue))

(event Input|AxisEvents|InputAxisLookUp
  (params (AxisValue :type Float%20%28single-precision%29))
  (Pawn|Input|AddControllerPitchInput AxisValue))

(fn ConstructionScript)

(fn GetWeaponSocket
  (params (socketName :type Name))
  (return (Transformation|GetSocketTransform (Variables|Default|GetheldWeapon) socketName "RTS_World")))

(fn PlayerSpawn
  (bind _outactors (Actor|GetAllActorsOfClass "humanCharacterBP_C"))
  (for _array_element _outactors
    (bind _output_get (Variables|Default|SetspawnLoc (Transformation|GetActorTransform _array_element)))
    (Transformation|SetActorTransform _output_get false true)))