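; Alien player character Blueprint for what appears to be a free-for-all mode, handling mouse look and end-of-match screens.
; On BeginPlay, the locally controlled instance binds to ffaGameState's OnWinPlayerFound, showing the win widget unless IsDead is set.
; DisplayDeathScreen sets that flag, removes HP bar widgets, shows the cursor and adds the death screen.
; PlayerSpawn, which teleports the alien to HumanCharacterBP transforms, is disconnected in the event graph.
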(event Custom|onWinPlayerFound_Event_0
  (if (not (Variables|Default|GetisDead))
    (bind _returnvalue (UserInterface|CreateWidget "/Game/Multiplayer/UI/playerWinScreenWidget.playerWinScreenWidget_C"))
    (UserInterface|Viewport|AddtoViewport _returnvalue 0)))

(event EventBeginPlay
  (if (Pawn|IsLocallyControlled)
    (bind _asffa_game_state (Utilities|Casting|CastToffaGameState (Game|GetGameState)))
    (EventDispatchers|BindEventtoOnWinPlayerFound _asffa_game_state (delegate Custom|onWinPlayerFound_Event_0))))

(event Collision|EventActorBeginOverlap
  (params (OtherActor :type Actor%20Object%20Reference)))

(event EventDisplayDeathScreen
  (Variables|Default|SetisDead true)
  (bind _foundwidgets (Widget|GetAllWidgetsOfClass "/Game/Multiplayer/playerHUD/playerHPbarWidget.playerHPbarWidget_C" false))
  (Widget|RemovefromParent _foundwidgets)
  (bind _returnvalue (UserInterface|CreateWidget "/Game/Multiplayer/UI/playerDeathScreenWidget.playerDeathScreenWidget_C"))
  (bind _output_get (Variables|Default|SetonDeathRef _returnvalue))
  (Variables|/Script/Engine.PlayerController|SetbShowMouseCursor (Game|GetPlayerController 0) true)
  (UserInterface|Viewport|AddtoViewport _output_get 0))

(event Input|AxisEvents|InputAxisTurn
  (params (AxisValue :type Float%20%28single-precision%29))
  (Variables|Default|SetbUseControllerRotationYaw true)
  (Pawn|Input|AddControllerYawInput AxisValue))

(event Input|AxisEvents|InputAxisLookUp
  (params (AxisValue :type Float%20%28single-precision%29))
  (Pawn|Input|AddControllerPitchInput AxisValue))

(fn ConstructionScript)

(fn PlayerSpawn
  (bind _outactors (Actor|GetAllActorsOfClass "/Game/Human/Blueprints/humanCharacterBP.humanCharacterBP_C"))
  (for _array_element _outactors
    (bind _output_get (Variables|Default|SetspawnLoc (Transformation|GetActorTransform _array_element)))
    (Transformation|SetActorTransform _output_get false true)))